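; BP_mainChar is the physics-driven main character, built around a Sphere component, with a speed boost on the S key.
; The boost fires only when SpeedTimer in kusaGameInstance has reached its threshold, then resets that timer.
; It adds an acceleration force scaled from current X velocity when already moving fast along +X, otherwise a fixed push along X.
; An angular impulse node is left unconnected and never runs.
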(event `self.ReceiveTick`
  (params (DeltaSeconds :type "Float (single-precision)")))

(event `Key|S`
  (params (Key :type "Key Structure"))
  (bind _sphere (`self.sphere`))
  (bind _x (.x (`SceneComponent.GetComponentVelocity` _sphere)))
  (:`Pressed`
    (bind _askusa_game_instance (cast `kusaGameInstance` (`GameplayStatics.GetGameInstance`)))
    (if (>= (`kusaGameInstance.SpeedTimer` _askusa_game_instance) 500.0)
      (set `kusaGameInstance.SpeedTimer` 0.0 _askusa_game_instance)
      (if (> _x 500.0)
        (`PrimitiveComponent.AddForce` _sphere (`KismetMathLibrary.MakeVector` (* _x 30.0) (.y (`SceneComponent.GetComponentVelocity` _sphere)) (.z (`SceneComponent.GetComponentVelocity` _sphere))) "None" true)
        (else
          (`PrimitiveComponent.AddForce` _sphere (100000.0 0.0 0.0) "None" true))))))

(fn `UserConstructionScript`)