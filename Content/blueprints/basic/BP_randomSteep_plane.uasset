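; BP_randomSteep_plane is an actor that randomly tilts one of its static mesh planes when play begins.
; BeginPlay switches on a random integer to choose one of nine mesh components, with one possible roll leaving all unchanged.
; The rotateIt event swaps the chosen mesh's first material to Ywlloe and adds a random relative pitch of up to 35 degrees.
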(event `self.ReceiveBeginPlay`
  (switch `int` (`KismetMathLibrary.RandomIntegerInRange` 0 9)
    (:`0`
      (`self.rotateIt` (`self.StaticMesh`)))
    (:`1`
      (`self.rotateIt` (`self.StaticMesh1`)))
    (:`2`
      (`self.rotateIt` (`self.StaticMesh2`)))
    (:`3`
      (`self.rotateIt` (`self.StaticMesh3`)))
    (:`4`
      (`self.rotateIt` (`self.StaticMesh4`)))
    (:`5`
      (`self.rotateIt` (`self.StaticMesh5`)))
    (:`6`
      (`self.rotateIt` (`self.StaticMesh6`)))
    (:`7`
      (`self.rotateIt` (`self.StaticMesh7`)))
    (:`8`
      (`self.rotateIt` (`self.StaticMesh8`)))))

(event `rotateIt`
  (params (mesh :type "StaticMeshComponent Object Reference (by ref)"))
  (`PrimitiveComponent.SetMaterial` mesh 0 "/Game/meshes/materials/ywlloe.ywlloe")
  (`SceneComponent.K2_AddRelativeRotation` mesh (`KismetMathLibrary.MakeRotator` 0.0 (`KismetMathLibrary.RandomFloatInRange` 0.0 35.0)) false false))

(fn `UserConstructionScript`)